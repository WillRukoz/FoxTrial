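; BP_PressureSwitch is a pressure plate that drives a linked DoorToActivate through box overlaps.
; Once EnableSwitch allows pressing, overlap calls SwitchActivated, turns the plate green and plays a timeline moving it along Z.
; Ending overlap deactivates the door, restores the material and reverses the timeline unless StayActive holds it, regardless of CanBePressed.
; ResetPlate restores the plate's material and height without notifying the door.
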(event `self.OverlapBox.OnComponentBeginOverlap`
  (params (OverlappedComponent :type "PrimitiveComponent Object Reference") (OtherActor :type "Actor Object Reference") (OtherComp :type "PrimitiveComponent Object Reference") (OtherBodyIndex :type Integer) (bFromSweep :type Boolean) (SweepResult :type "HitResult Structure (by ref)"))
  (`PrimitiveComponent.SetMaterial` (`self.Switch`) 0 "/Game/ProyectDoor/Materials/M_BotonVerde.M_BotonVerde")
  (if (`self.CanBePressed`)
    (`/Game/LevelDesing/BP_Door.SwitchActivated` (`self.DoorToActivate`))
    (bind (_direction _switchposition) (`Timeline|SwitchActivate` :!label _label)
      (:`Update`
        (`SceneComponent.K2_SetRelativeLocation` (`self.Switch`) (`KismetMathLibrary.MakeVector` 0.0 0.0 _switchposition) false false)))
    (else
      (`PrimitiveComponent.SetMaterial` (`self.Switch`) 0 "/Game/LevelDesing/M_Boton_Interactivo.M_Boton_Interactivo"))))

(event `EnableSwitch`
  (set `self.CanBePressed` true))

(event `self.OverlapBox.OnComponentEndOverlap`
  (params (OverlappedComponent :type "PrimitiveComponent Object Reference") (OtherActor :type "Actor Object Reference") (OtherComp :type "PrimitiveComponent Object Reference") (OtherBodyIndex :type Integer))
  (`PrimitiveComponent.SetMaterial` (`self.Switch`) 0 "/Game/LevelDesing/M_Boton_Interactivo.M_Boton_Interactivo")
  (if (`self.StayActive`)
    (`PrimitiveComponent.SetMaterial` (`self.Switch`) 0 "/Game/ProyectDoor/Materials/M_BotonVerde.M_BotonVerde")
    (else
      (`/Game/LevelDesing/BP_Door.SwitchDeactivated` (`self.DoorToActivate`))
      (goto _label :!via `Reverse`))))

(fn `ResetPlate`
  (set `self.IsPressed` false)
  (if (not (`self.StayActive`))
    (set `self.StayActive` false))
  (`PrimitiveComponent.SetMaterial` (`self.Switch`) 0 "/Game/LevelDesing/M_Boton_Interactivo.M_Boton_Interactivo")
  (`SceneComponent.K2_SetRelativeLocation` (`self.Switch`) (0.0 0.0 8.0) false false))

(fn `UserConstructionScript`)