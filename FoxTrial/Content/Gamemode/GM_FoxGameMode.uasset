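; Game mode for the Fox game that runs a countdown from a time limit and defines win and lose states.
; BeginPlay creates a dynamic vignette material and adds it to the first post process volume found, at zero weight.
; Tick lowers the timer, sets a constant vignette opacity and calls LoseGame only on exactly zero.
; WinGame, uncalled here, and LoseGame set GameOver and print Spanish result messages.
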(event `self.ReceiveBeginPlay`
  ; Set Timer and vignette
  (set `self.TimeRemaining` (`self.TimeLimit`))
  (bind _returnvalue (`KismetMaterialLibrary.CreateDynamicMaterialInstance` "/Game/Art/Material/MI_VignetteInst.MI_VignetteInst"))
  (bind _output_get (set `self.VignetteMaterial` _returnvalue))
  (bind _outactors (`GameplayStatics.GetAllActorsOfClass` "/Script/Engine.PostProcessVolume"))
  (bind _output_get_2 (set `self.PostProcessVolume` (`|GetArrayItem` _outactors)))
  (`PostProcessVolume.AddOrUpdateBlendable` _output_get_2 _output_get 0.0))

(event `self.ReceiveTick`
  (params (DeltaSeconds :type "Float (single-precision)"))
  (if (!= (`self.bGameOver`) true)
    (set `self.TimeRemaining` (- (`self.TimeRemaining`) DeltaSeconds))
    (`MaterialInstanceDynamic.SetScalarParameterValue` (`self.VignetteMaterial`) "Opacity" 50.0)
    (if (== (`self.TimeRemaining`) 0.0)
      (`self.LoseGame`))))

(fn `LoseGame`
  (set `self.bGameOver` true)
  (`KismetSystemLibrary.PrintString` "PERDISTE"))

(fn `UserConstructionScript`)

(fn `WinGame`
  (set `self.bGameOver` true)
  (`KismetSystemLibrary.PrintString` "GANASTE"))