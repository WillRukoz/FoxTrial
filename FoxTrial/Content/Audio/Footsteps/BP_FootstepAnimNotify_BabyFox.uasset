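; Anim notify that plays footstep sounds for the baby fox, acting only when the mesh owner is a BP_FoxBaby.
; A downward line trace from the owner reads the physical surface and picks a grass, metal, wood or snow sound, with dog footsteps for floor and other surfaces.
; Sounds play at world origin rather than at the fox, and the volume select is hard-wired to full.
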(fn `Received_Notify`
  (params (MeshComp :type "SkeletalMeshComponent Object Reference") (Animation :type "AnimSequenceBase Object Reference") (EventReference :type "AnimNotifyEventReference Structure (by ref)"))
  (returns (ReturnValue :type Boolean))
  (bind _returnvalue (`KismetMathLibrary.SelectFloat` 0.5 1.0))
  (bind _returnvalue_2 (`ActorComponent.GetOwner` MeshComp))
  (bind _returnvalue_3 (`Actor.K2_GetActorLocation` _returnvalue_2))
  (cast `/Game/Characters/Fox/BabyFox/BP_FoxBaby` _returnvalue_2)
  (bind (_outhit _returnvalue_4) (`KismetSystemLibrary.LineTraceSingle` _returnvalue_3 (+ _returnvalue_3 (* (`Actor.GetActorUpVector` _returnvalue_2) -200.0)) "TraceTypeQuery3"))
  (if _returnvalue_4
    (switch `EPhysicalSurface` (`GameplayStatics.GetSurfaceType` _outhit)
      (:`SurfaceType_Default`
        (`GameplayStatics.PlaySoundAtLocation` "/Game/Audio/Footsetps/Dog_Footsteps_3.Dog_Footsteps_3" (0.0 0.0 0.0) (struct) _returnvalue 1.0 0.0 null null null null))
      (:`SurfaceType1`
        (`GameplayStatics.PlaySoundAtLocation` "/Game/Audio/Footsteps/Audio/A_GrassFootstep.A_GrassFootstep" (0.0 0.0 0.0) (struct) _returnvalue 1.0 0.0 null null null null)
        (return false))
      (:`SurfaceType2`
        (`GameplayStatics.PlaySoundAtLocation` "/Game/Audio/Footsteps/Audio/A_MetalFootstep.A_MetalFootstep" (0.0 0.0 0.0) (struct) _returnvalue 1.0 0.0 null null null null)
        (return false))
      (:`SurfaceType3`
        (`GameplayStatics.PlaySoundAtLocation` "/Game/Audio/Footsteps/Audio/A_WoodFootstep.A_WoodFootstep" (0.0 0.0 0.0) (struct) _returnvalue 1.0 0.0 null null null null)
        (return false))
      (:`SurfaceType4`
        (`GameplayStatics.PlaySoundAtLocation` "/Game/Audio/Footsetps/Footsteps_Snow__Walking_.Footsteps_Snow__Walking_" (0.0 0.0 0.0) (struct) _returnvalue 1.0 0.0 null null null null)
        (return false))
      (:`SurfaceType5`
        (`GameplayStatics.PlaySoundAtLocation` "/Game/Audio/Footsetps/Dog_Footsteps_3.Dog_Footsteps_3" (0.0 0.0 0.0) (struct) _returnvalue 1.0 0.0 null null null null)
        (return false)))
    (else
      (return false))))