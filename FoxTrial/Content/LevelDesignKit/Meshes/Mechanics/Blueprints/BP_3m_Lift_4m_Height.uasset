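; Lift Blueprint for the level design kit that raises a floor platform automatically on BeginPlay and later sends it back.
; The LiftTravel timeline drives Floor4x4m's relative location.
; A ten-second Delay in the timeline update precedes a top-height check, which clears Up and reverses the timeline.
; Despite a note mentioning the E key, no input is wired, so the FlipFlop's reverse branch stays unused.
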(event `self.ReceiveBeginPlay`
  ; Mueve con la E
  (`/Engine/EditorBlueprintResources/StandardMacros.FlipFlop`
    (:`A`
      (set `self.Up` true)
      (bind (_direction _newtrack_1) (`Timeline|LiftTravel` :!label _label)
        (:`Update`
          (`SceneComponent.K2_SetRelativeLocation` (`self.Floor4x4m`) _newtrack_1 false false)
          (`KismetSystemLibrary.Delay` 10.0)
          (if (and (== (.z (.location (`SceneComponent.GetRelativeTransform` (`self.Floor4x4m`)))) 500.0) (`self.Up`))
            (set `self.Up` false :!label _label_2)
            (goto _label :!via `Reverse`)))))
    (:`B`
      (goto _label_2))))

(fn `UserConstructionScript`)