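; AI controller for NPCs that runs the BT_NPC behavior tree and reacts to AI perception updates.
; Each stimulus sets the Investigating Blackboard bool from whether sensing succeeded and prints the sense class name.
; A sensed player becomes TargetLocationActor and starts detection on BP_FoxCharacter.
; A lost fox character stops detection, stores the stimulus location in LocationV and clears the target actor.
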(event `self.ReceiveBeginPlay`
  ; Inicializa behavior tree
  (`self.RunBehaviorTree` "/Game/EnemyAI/Behaiviour/BT_NPC.BT_NPC"))

(event `self.AIPerception.OnTargetPerceptionUpdated`
  (params (Actor :type "Actor Object Reference") (Stimulus :type "AIStimulus Structure"))
  ; TargetPerception, deteccion de jugador e inicializador de ui
  (bind _returnvalue (`AIPerceptionSystem.GetSenseClassForStimulus` Stimulus))
  (`self.HandleSense` (`KismetSystemLibrary.GetClassDisplayName` _returnvalue) Stimulus Actor))

(fn `HandleSense`
  (params (InString :type String) (Stimul :type "AIStimulus Structure") (`Sensed Actor` :type "Actor Object Reference"))
  (bind (_stimul_age _stimul_expirationage _stimul_strength _stimul_stimuluslocation) (break `AIStimulus` (`local.Stimul`)))
  (bind (_stimul_age_2 _stimul_expirationage_2 _stimul_strength_2 _stimul_stimuluslocation_2 _stimul_receiverlocation _stimul_tag _stimul_bsuccessfullysensed) (break `AIStimulus` (`local.Stimul`)))
  ; Llamado al bool de la blackboard
  (`KismetSystemLibrary.PrintString` InString)
  (`BlackboardComponent.SetValueAsBool` (`self.Blackboard`) "Investigating" _stimul_bsuccessfullysensed)
  (if _stimul_bsuccessfullysensed
    ; Deteccion Del Player
    (if (== (`local.Sensed Actor`) (`GameplayStatics.GetPlayerCharacter` 0))
      (bind _asbp_fox_character (cast `/Game/Characters/Fox/BP_FoxCharacter` (`local.Sensed Actor`)))
      (`/Game/Characters/Fox/BP_FoxCharacter.StartDetection` _asbp_fox_character true)
      (`KismetSystemLibrary.PrintString` "sensed player")
      (`BlackboardComponent.SetValueAsObject` (`self.Blackboard`) "TargetLocationActor" (`local.Sensed Actor`)))
    (else
      ; Deteccion del ultimo lugar del player
      (bind _asbp_fox_character_2 (cast `/Game/Characters/Fox/BP_FoxCharacter` (`local.Sensed Actor`)))
      (`/Game/Characters/Fox/BP_FoxCharacter.StartDetection` _asbp_fox_character_2 false)
      (`BlackboardComponent.SetValueAsVector` (`self.Blackboard`) "LocationV" _stimul_stimuluslocation)
      (`BlackboardComponent.SetValueAsObject` (`self.Blackboard`) "TargetLocationActor" null))))

(fn `UserConstructionScript`)