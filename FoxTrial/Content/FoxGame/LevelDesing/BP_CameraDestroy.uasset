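; BP_CameraDestroy is an interactable button that triggers a linked CCTV camera, apparently to destroy it, and can enable a pressure switch.
; Overlapping component R shows or hides its prompt widget.
; Interact calls EnableSwitch on any valid BPPressureSwitch and always calls Interact on BPCCTV without a validity check.
; It also turns the button green, removes the widget and plays a click through DoOnce gates.
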(event `self.Interact`
  (`|ExecutionSequence`
    (:`then_0`
      (bind _bp_pressureswitch (`self.BP_PressureSwitch`)
        (:`then`
          (`/Game/FoxGame/LevelDesing/BP_PressureSwitch.EnableSwitch` _bp_pressureswitch)
          (`PrimitiveComponent.SetMaterial` (`self.BotonMesh`) 0 "/Game/FoxGame/Blueprints/SlidingDoor/Materials/M_GreenButton.M_GreenButton")
          (`ActorComponent.K2_DestroyComponent` (`self.Widget`))
          (`/Engine/EditorBlueprintResources/StandardMacros.DoOnce` false
            (:`Completed`
              (`GameplayStatics.PlaySoundAtLocation` "/Engine/VREditor/Sounds/VR_click1.VR_click1" (`SceneComponent.K2_GetComponentLocation` (`self.BotonMesh`)) (struct) 1.0 1.0 0.0 null null null null))))
        (:`else`)))
    (:`then_1`
      (`/Game/FoxGame/LevelDesing/BPI_InterectInterface.Interact` (`self.BP_CCTV `))
      (`PrimitiveComponent.SetMaterial` (`self.BotonMesh`) 0 "/Game/FoxGame/Blueprints/SlidingDoor/Materials/M_GreenButton.M_GreenButton")
      (bind _widget (`self.Widget`)
        (:`then`
          (`ActorComponent.K2_DestroyComponent` _widget)
          (set `self.bJugadorCerca` true)
          (`/Engine/EditorBlueprintResources/StandardMacros.DoOnce` false
            (:`Completed`
              (`GameplayStatics.PlaySoundAtLocation` "/Engine/VREditor/Sounds/VR_click1.VR_click1" (`SceneComponent.K2_GetComponentLocation` (`self.BotonMesh`)) (struct) 1.0 1.0 0.0 null null null null))))
        (:`else`)))))

(event `self.R.OnComponentBeginOverlap`
  (params (OverlappedComponent :type "PrimitiveComponent Object Reference") (OtherActor :type "Actor Object Reference") (OtherComp :type "PrimitiveComponent Object Reference") (OtherBodyIndex :type Integer) (bFromSweep :type Boolean) (SweepResult :type "HitResult Structure (by ref)"))
  (bind _widget (`self.Widget`)
    (:`then`
      (`SceneComponent.SetVisibility` _widget true false))
    (:`else`)))

(event `self.R.OnComponentEndOverlap`
  (params (OverlappedComponent :type "PrimitiveComponent Object Reference") (OtherActor :type "Actor Object Reference") (OtherComp :type "PrimitiveComponent Object Reference") (OtherBodyIndex :type Integer))
  (bind _widget (`self.Widget`)
    (:`then`
      (`SceneComponent.SetVisibility` _widget false false))
    (:`else`)))

(fn `UserConstructionScript`)