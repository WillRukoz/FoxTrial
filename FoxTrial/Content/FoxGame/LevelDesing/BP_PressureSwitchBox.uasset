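; Pressure switch that triggers a linked door when an actor tagged CajaTrigger overlaps it while it can be pressed.
; Pressing plays timelines that lower the switch, disable the box's physics and lerp it onto the overlap box with zeroed rotation.
; A movable box leaving releases the switch and door unless StayActive is set.
; Switch materials reflect state; EnableSwitch makes it pressable, and ResetPlate restores material and height.
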(event `ColorUpdate`
  (if (`self.CanBePressed`) :!label _label
    (`PrimitiveComponent.SetMaterial` (`self.Switch`) 0 "/Game/Art/Material/Button/M_InteractiveButton.M_InteractiveButton")
    (else
      (`PrimitiveComponent.SetMaterial` (`self.Switch`) 0 "/Game/Art/Material/Button/M_Bottunt.M_Bottunt")
      (`ActorComponent.Activate` (`self.OverlapBox`) false))))

(event `self.ReceiveBeginPlay`
  (goto _label))

(event `self.OverlapBox.OnComponentBeginOverlap`
  (params (OverlappedComponent :type "PrimitiveComponent Object Reference") (OtherActor :type "Actor Object Reference") (OtherComp :type "PrimitiveComponent Object Reference") (OtherBodyIndex :type Integer) (bFromSweep :type Boolean) (SweepResult :type "HitResult Structure (by ref)"))
  (bind _returnvalue (`self.GetComponentByClass` (`self.Box`) "/Script/Engine.StaticMeshComponent"))
  (if (and (`self.ActorHasTag` OtherActor "CajaTrigger") (stale `EnableSwitch` _output_get)) :!label _label_2
    (set `self.Box` OtherActor)
    (`PrimitiveComponent.SetMaterial` (`self.Switch`) 0 "/Game/FoxGame/Blueprints/SlidingDoor/Materials/M_GreenButton.M_GreenButton")
    (if (`self.CanBePressed`)
      (`/Game/FoxGame/LevelDesing/BP_Door.SwitchActivated` (`self.DoorToActivate`))
      (bind (_direction _switchposition) (`Timeline|SwitchActivate` :!label _label_3)
        (:`Update`
          (`SceneComponent.K2_SetRelativeLocation` (`self.Switch`) (`KismetMathLibrary.MakeVector` 0.0 0.0 _switchposition) false false)
          (`PrimitiveComponent.SetSimulatePhysics` _returnvalue false)
          (bind _output_get (set `self.StartLocation` (`SceneComponent.K2_GetComponentLocation` _returnvalue)))
          (bind _output_get_2 (set `self.TargetLocation ` (`SceneComponent.K2_GetComponentLocation` (`self.OverlapBox`))))
          (bind (_direction_2 _alpha) (`Timeline|BoxToFix`)
            (:`Update`
              (bind (_returnvalue_x _returnvalue_y _returnvalue_z) (`KismetMathLibrary.BreakVector` (`KismetMathLibrary.VLerp` _output_get _output_get_2 _alpha)))
              (`SceneComponent.K2_SetRelativeLocation` _returnvalue (`KismetMathLibrary.MakeVector` _returnvalue_x _returnvalue_y _returnvalue_z) false false)
              (`SceneComponent.K2_SetWorldRotation` _returnvalue (`KismetMathLibrary.MakeRotator` 0.0) false false)))))
      (else
        (`PrimitiveComponent.SetMaterial` (`self.Switch`) 0 "/Game/Art/Material/Button/M_InteractiveButton.M_InteractiveButton")))))

(event `EnableSwitch`
  (bind _output_get (set `self.CanBePressed` true))
  (goto _label_2))

(event `self.OverlapBox.OnComponentEndOverlap`
  (params (OverlappedComponent :type "PrimitiveComponent Object Reference") (OtherActor :type "Actor Object Reference") (OtherComp :type "PrimitiveComponent Object Reference") (OtherBodyIndex :type Integer))
  (cast `/Game/FoxGame/LevelDesing/BP_MovableBox` OtherActor)
  (if (stale `EnableSwitch` _output_get)
    (`PrimitiveComponent.SetMaterial` (`self.Switch`) 0 "/Game/Art/Material/Button/M_InteractiveButton.M_InteractiveButton")
    (if (`self.StayActive`)
      (`PrimitiveComponent.SetMaterial` (`self.Switch`) 0 "/Game/FoxGame/Blueprints/SlidingDoor/Materials/M_GreenButton.M_GreenButton")
      (else
        (`/Game/FoxGame/LevelDesing/BP_Door.SwitchDeactivated` (`self.DoorToActivate`))
        (goto _label_3 :!via `Reverse`)))))

(fn `ResetPlate`
  (set `self.IsPressed` false)
  (if (not (`self.StayActive`))
    (set `self.StayActive` false))
  (`PrimitiveComponent.SetMaterial` (`self.Switch`) 0 "/Game/Art/Material/Button/M_InteractiveButton.M_InteractiveButton")
  (`SceneComponent.K2_SetRelativeLocation` (`self.Switch`) (0.0 0.0 8.0) false false))

(fn `UserConstructionScript`)