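; Final level door that slides on a timeline and leads to the credits level.
; Switch activation and deactivation events adjust a counter, playing the timeline when the required count is met and reversing it otherwise.
; The timeline's Update moves the door and also spawns the fade-out widget, then loads Level_Credits after a delay.
; BP_FoxBaby overlapping ResetPlate resets any associated button and reverses the door; IsDoorAllowedToOpen is unused.
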(event `self.ReceiveActorBeginOverlap`
  (params (OtherActor :type "Actor Object Reference"))
  ; TODO
  (cast `/Game/ThirdPerson/Blueprints/BP_ThirdPersonCharacter` OtherActor))

(event `SwitchActivated`
  (`/Engine/EditorBlueprintResources/StandardMacros.IncrementInt` (`self.PressureSwitchesActive`)
    (:`  `
      (if (>= (`self.PressureSwitchesActive`) (`self.PressureSwitchesNeeded`))
        (bind (_direction _doorposition) (`Timeline|DoorActivation` :!label _label)
          (:`Update`
            (`SceneComponent.K2_SetRelativeLocation` (`self.Door`) (`KismetMathLibrary.MakeVector` 0.0 0.0 _doorposition) false false)
            (bind _returnvalue (`|CreateWidget` "/Game/UI/WBP_GameFade.WBP_GameFade_C"))
            (bind _output_get (set `self.GameFade` _returnvalue))
            (`UserWidget.AddToViewport` _output_get 0)
            (`UserWidget.PlayAnimation` (`self.GameFade`) (`/Game/UI/WBP_GameFade.FadeOut` (`self.GameFade`)) 0.0 1 "Forward" 0.5 false)
            (`KismetSystemLibrary.Delay` 3.0)
            (`GameplayStatics.OpenLevel` "Level_Credits")))
        (else
          (goto _label :!via `Reverse`))))))

(event `SwitchDeactivated`
  (`/Engine/EditorBlueprintResources/StandardMacros.DecrementInt` (`self.PressureSwitchesActive`)
    (:`  `
      (if (>= (`self.PressureSwitchesActive`) (`self.PressureSwitchesNeeded`))
        (goto _label)
        (else
          (goto _label :!via `Reverse`))))))

(event `self.ResetPlate.OnComponentBeginOverlap`
  (params (OverlappedComponent :type "PrimitiveComponent Object Reference") (OtherActor :type "Actor Object Reference") (OtherComp :type "PrimitiveComponent Object Reference") (OtherBodyIndex :type Integer) (bFromSweep :type Boolean) (SweepResult :type "HitResult Structure (by ref)"))
  (cast `/Game/Characters/Fox/BabyFox/BP_FoxBaby` OtherActor)
  (`self.ButtonAssociate`
    (:`then`
      (`/Game/FoxGame/LevelDesing/BP_PressureSwitch.ResetPlate` (`self.ButtonAssociate`))
      (goto _label :!via `Reverse`))
    (:`else`
      (goto _label :!via `Reverse`))))

(fn `IsDoorAllowedToOpen`
  (returns (ReturnValue :type Boolean))
  (return (and (`self.ButtonPressed`) (>= (`self.PressureSwitchesActive`) (`self.PressureSwitchesNeeded`)))))

(fn `UserConstructionScript`)