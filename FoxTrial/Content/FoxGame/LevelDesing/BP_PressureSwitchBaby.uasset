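; BP_PressureSwitchBaby is a floor pressure switch that signals a linked door and a final door when something overlaps it.
; If pressable, overlap turns it green, activates both doors and moves the switch via a timeline; leaving reverses this unless StayActive is set.
; CanBePressed gates interaction and sets the initial material, EnableSwitch unlocks it, and ResetPlate restores the idle material and height.
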(event `ColorUpdate`
  (if (`self.CanBePressed`) :!label _label
    (`PrimitiveComponent.SetMaterial` (`self.Switch`) 0 "/Game/Art/Material/Button/M_InteractiveButton.M_InteractiveButton")
    (else
      (`PrimitiveComponent.SetMaterial` (`self.Switch`) 0 "/Game/Art/Material/Button/M_Bottunt.M_Bottunt")
      (`ActorComponent.Activate` (`self.OverlapBox`) false))))

(event `self.ReceiveBeginPlay`
  (goto _label))

(event `self.OverlapBox.OnComponentBeginOverlap`
  (params (OverlappedComponent :type "PrimitiveComponent Object Reference") (OtherActor :type "Actor Object Reference") (OtherComp :type "PrimitiveComponent Object Reference") (OtherBodyIndex :type Integer) (bFromSweep :type Boolean) (SweepResult :type "HitResult Structure (by ref)"))
  (if (stale `EnableSwitch` _output_get)
    (`PrimitiveComponent.SetMaterial` (`self.Switch`) 0 "/Game/FoxGame/Blueprints/SlidingDoor/Materials/M_GreenButton.M_GreenButton")
    (if (`self.CanBePressed`)
      (`/Game/FoxGame/LevelDesing/BP_Door.SwitchActivated` (`self.DoorToActivate`))
      (`/Game/FoxGame/LevelDesing/BP_DoorFinal.SwitchActivated` (`self.FinalDoor`))
      (bind (_direction _switchposition) (`Timeline|SwitchActivate` :!label _label_2)
        (:`Update`
          (`SceneComponent.K2_SetRelativeLocation` (`self.Switch`) (`KismetMathLibrary.MakeVector` 0.0 0.0 _switchposition) false false)))
      (else
        (`PrimitiveComponent.SetMaterial` (`self.Switch`) 0 "/Game/Art/Material/Button/M_InteractiveButton.M_InteractiveButton")))))

(event `EnableSwitch`
  (bind _output_get (set `self.CanBePressed` true)))

(event `self.OverlapBox.OnComponentEndOverlap`
  (params (OverlappedComponent :type "PrimitiveComponent Object Reference") (OtherActor :type "Actor Object Reference") (OtherComp :type "PrimitiveComponent Object Reference") (OtherBodyIndex :type Integer))
  (if (stale `EnableSwitch` _output_get)
    (`PrimitiveComponent.SetMaterial` (`self.Switch`) 0 "/Game/Art/Material/Button/M_InteractiveButton.M_InteractiveButton")
    (if (`self.StayActive`)
      (`PrimitiveComponent.SetMaterial` (`self.Switch`) 0 "/Game/FoxGame/Blueprints/SlidingDoor/Materials/M_GreenButton.M_GreenButton")
      (else
        (`/Game/FoxGame/LevelDesing/BP_Door.SwitchDeactivated` (`self.DoorToActivate`))
        (`/Game/FoxGame/LevelDesing/BP_DoorFinal.SwitchDeactivated` (`self.FinalDoor`))
        (goto _label_2 :!via `Reverse`)))))

(fn `ResetPlate`
  (set `self.IsPressed` false)
  (if (not (`self.StayActive`))
    (set `self.StayActive` false))
  (`PrimitiveComponent.SetMaterial` (`self.Switch`) 0 "/Game/Art/Material/Button/M_InteractiveButton.M_InteractiveButton")
  (`SceneComponent.K2_SetRelativeLocation` (`self.Switch`) (0.0 0.0 8.0) false false))

(fn `UserConstructionScript`)