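; BP_ChangeCamera is a trigger volume that switches the player fox between third-person and first-person views.
; When the player character enters the Box, it activates the fox's first-person camera, deactivates the third-person one and hides the character mesh.
; Leaving the Box reverses all three changes, and both events print a debug "Detected" message.
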(event `self.Box.OnComponentBeginOverlap`
  (params (OverlappedComponent :type "PrimitiveComponent Object Reference") (OtherActor :type "Actor Object Reference") (OtherComp :type "PrimitiveComponent Object Reference") (OtherBodyIndex :type Integer) (bFromSweep :type Boolean) (SweepResult :type "HitResult Structure (by ref)"))
  (bind _returnvalue (`GameplayStatics.GetPlayerCharacter` 0))
  (if (== OtherActor _returnvalue)
    (bind _asbp_fox_character (cast `/Game/Characters/Fox/BP_FoxCharacter` _returnvalue))
    (`KismetSystemLibrary.PrintText` "Detected")
    (`ActorComponent.SetActive` (`/Game/Characters/Fox/BP_FoxCharacter.FirstPersonCamera` _asbp_fox_character) true false)
    (`ActorComponent.SetActive` (`/Game/Characters/Fox/BP_FoxCharacter.ThirdPersonCamera` _asbp_fox_character) false false)
    (`SceneComponent.SetVisibility` (`Character.Mesh` _asbp_fox_character) false false)))

(event `self.Box.OnComponentEndOverlap`
  (params (OverlappedComponent :type "PrimitiveComponent Object Reference") (OtherActor :type "Actor Object Reference") (OtherComp :type "PrimitiveComponent Object Reference") (OtherBodyIndex :type Integer))
  (bind _returnvalue (`GameplayStatics.GetPlayerCharacter` 0))
  (if (== OtherActor _returnvalue)
    (bind _asbp_fox_character (cast `/Game/Characters/Fox/BP_FoxCharacter` _returnvalue))
    (`KismetSystemLibrary.PrintText` "Detected")
    (`ActorComponent.SetActive` (`/Game/Characters/Fox/BP_FoxCharacter.FirstPersonCamera` _asbp_fox_character) false false)
    (`ActorComponent.SetActive` (`/Game/Characters/Fox/BP_FoxCharacter.ThirdPersonCamera` _asbp_fox_character) true false)
    (`SceneComponent.SetVisibility` (`Character.Mesh` _asbp_fox_character) true false)))

(fn `UserConstructionScript`)