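; Trigger volume that smoothly turns the fox character's camera toward a focus location, once, when it enters the box.
; The first overlap plays a timeline that interpolates control rotation toward a look-at rotation from the character to the FocusLocation coordinates.
; An optional SlowPlayer flag lowers walk speed during the refocus, then sets it back to a fixed value after a delay.
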(event `self.Box.OnComponentBeginOverlap`
  (params (OverlappedComponent :type "PrimitiveComponent Object Reference") (OtherActor :type "Actor Object Reference") (OtherComp :type "PrimitiveComponent Object Reference") (OtherBodyIndex :type Integer) (bFromSweep :type Boolean) (SweepResult :type "HitResult Structure (by ref)"))
  (bind _charactermovement (`Character.CharacterMovement` (`self.As BP Fox Character`)))
  ; SmoothCameraRefocus}
  (bind _asbp_fox_character (cast `/Game/Characters/Fox/BP_FoxCharacter` OtherActor))
  (set `self.As BP Fox Character` _asbp_fox_character)
  (`/Engine/EditorBlueprintResources/StandardMacros.DoOnce` false
    (:`Completed`
      (`Timeline|Timeline`
        (:`Update`
          (`Controller.SetControlRotation` (`GameplayStatics.GetPlayerController` 0) (`KismetMathLibrary.RInterpTo` (`Pawn.GetControlRotation` _asbp_fox_character) (`KismetMathLibrary.FindLookAtRotation` (`self.K2_GetActorLocation` _asbp_fox_character) (`KismetMathLibrary.MakeVector` (`self.TargetX`) (`self.TargetY`) (`self.TargetZ`))) (`GameplayStatics.GetWorldDeltaSeconds`) 2.0))
          (if (`self.SlowPlayer`)
            (set `CharacterMovementComponent.MaxWalkSpeed` 100.0 _charactermovement)
            (`KismetSystemLibrary.Delay` 5.0)
            (set `CharacterMovementComponent.MaxWalkSpeed` 300.0 _charactermovement)))))))

(fn `UserConstructionScript`)