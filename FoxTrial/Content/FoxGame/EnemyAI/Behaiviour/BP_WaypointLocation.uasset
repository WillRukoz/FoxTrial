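; Behaviour tree task that walks a BP_Guard to the current waypoint on its path.
; It sets the guard's walk speed, waits for the guard's WaitTime, then runs AIMoveTo toward that waypoint.
; On success it zeroes the blackboard target vector, rotates the guard to the waypoint's facing and finishes.
; The waypoint index is not advanced here, and a failed cast or move never calls FinishExecute.
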(event `self.ReceiveExecuteAI`
  (params (OwnerController :type "AIController Object Reference") (ControlledPawn :type "Pawn Object Reference"))
  ; AI move to a los Waypoints
  (bind _asbp_guard (cast `/Game/FoxGame/EnemyAI/Blueprints/BP_Guard` ControlledPawn))
  (bind _output_get (set `self.As BP Scientist` _asbp_guard))
  (set `CharacterMovementComponent.MaxWalkSpeed` (`self.WalkSpeed`) (`Character.CharacterMovement` _output_get))
  (`KismetSystemLibrary.Delay` (`/Game/FoxGame/EnemyAI/Blueprints/BP_Guard.WaitTime` _output_get))
  (bind _output (`|GetArrayItem` (`/Game/FoxGame/EnemyAI/Blueprints/BP_Guard.Path` _output_get) (`/Game/FoxGame/EnemyAI/Blueprints/BP_Guard.CurrentWaypoint` _output_get)))
  (`|AIMoveTo` _output_get (0.0 0.0 0.0) _output
    (:`OnSuccess`
      (`BTFunctionLibrary.SetBlackboardValueAsVector` (`self.BB_targetVector`))
      (bind _rootcomponent (`Actor.RootComponent` _output_get))
      (`KismetSystemLibrary.MoveComponentTo` _rootcomponent (`SceneComponent.K2_GetComponentLocation` _rootcomponent) (`Actor.K2_GetActorRotation` _output) false false 0.2 true)
      (`self.FinishExecute` true))))