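; BP_FinishedPatrol is an AI behavior tree task that updates a guard's waypoint along its patrol path.
; If the next index is valid, it advances only when the scientist child's ShouldMove flag is set, printing debug text.
; At path ends, PathBehavior wraps to the start, stays still or reverses direction.
; Pawns failing the BP_Guard or BP_Scientist_Child cast never finish the task.
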(event `self.ReceiveExecuteAI`
  (params (OwnerController :type "AIController Object Reference") (ControlledPawn :type "Pawn Object Reference"))
  (bind _as_bp_guard (`self.As BP_Guard`))
  (bind _as_bp_guard_2 (`self.As BP_Guard`))
  (bind _asbp_guard (cast `/Game/FoxGame/EnemyAI/Blueprints/BP_Guard` ControlledPawn))
  (bind _output_get (set `self.As BP_Guard` _asbp_guard))
  (bind _asbp_scientist_child (cast `/Game/FoxGame/EnemyAI/Blueprints/BP_Scientist_Child` _output_get))
  (if (`KismetArrayLibrary.Array_IsValidIndex` (`/Game/FoxGame/EnemyAI/Blueprints/BP_Guard.Path` _output_get) (+ (`/Game/FoxGame/EnemyAI/Blueprints/BP_Guard.CurrentWaypoint` _output_get) (`/Game/FoxGame/EnemyAI/Blueprints/BP_Guard.Direction` _output_get)))
    (if (`/Game/FoxGame/EnemyAI/Blueprints/BP_Scientist_Child.ShouldMove` _asbp_scientist_child)
      (`KismetSystemLibrary.PrintString` "IsTrue")
      (set `/Game/FoxGame/EnemyAI/Blueprints/BP_Guard.CurrentWaypoint` (+ (`/Game/FoxGame/EnemyAI/Blueprints/BP_Guard.CurrentWaypoint` _as_bp_guard_2) (`/Game/FoxGame/EnemyAI/Blueprints/BP_Guard.Direction` _as_bp_guard_2)) _as_bp_guard_2)
      (`self.FinishExecute` true)
      (else
        (`KismetSystemLibrary.PrintString` "IsFalse")
        (`self.FinishExecute` true)))
    (else
      (switch `/Game/FoxGame/EnemyAI/Blueprints/PatrolEnd` (`/Game/FoxGame/EnemyAI/Blueprints/BP_Guard.PathBehavior` (`self.As BP_Guard`))
        (:`NewEnumerator0`
          (set `/Game/FoxGame/EnemyAI/Blueprints/BP_Guard.CurrentWaypoint` 0 (`self.As BP_Guard`))
          (`self.FinishExecute` true))
        (:`NewEnumerator1`
          (`self.FinishExecute` true))
        (:`NewEnumerator3`
          (set `/Game/FoxGame/EnemyAI/Blueprints/BP_Guard.Direction` (* (`/Game/FoxGame/EnemyAI/Blueprints/BP_Guard.Direction` _as_bp_guard) -1) _as_bp_guard)
          (`self.FinishExecute` true))))))