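; BP_Guard is an enemy guard that hurts the player's fox on contact and emits periodic idle sounds.
; Its Death collider applies damage to BP_FoxCharacter when the player pawn begins overlapping it, with a debug print on each hit.
; A looping timer plays the idle sound at the guard's location, using an interval randomized once at BeginPlay, so each guard keeps its own fixed rhythm.
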(event `self.Death.OnComponentBeginOverlap`
  (params (OverlappedComponent :type "PrimitiveComponent Object Reference") (OtherActor :type "Actor Object Reference") (OtherComp :type "PrimitiveComponent Object Reference") (OtherBodyIndex :type Integer) (bFromSweep :type Boolean) (SweepResult :type "HitResult Structure (by ref)"))
  (bind _returnvalue (`GameplayStatics.GetPlayerPawn` 0))
  ; DeathBox collider
  (if (== OtherActor _returnvalue)
    (`KismetSystemLibrary.PrintString` "hit")
    (bind _asbp_fox_character (cast `/Game/Characters/Fox/BP_FoxCharacter` _returnvalue))
    (`GameplayStatics.ApplyDamage` _asbp_fox_character 1.0)))

(event `self.ReceiveBeginPlay`
  (`KismetSystemLibrary.K2_SetTimerDelegate` (delegate `IdleSounds`) (`KismetMathLibrary.RandomFloatInRange` 10.0 20.0) true))

(event `IdleSounds`
  (`GameplayStatics.PlaySoundAtLocation` "/Game/Audio/Guards/Idle/SQ_GuardIdle.SQ_GuardIdle" (`self.K2_GetActorLocation`) (struct) 1.0 1.0 0.0 null null null null))

(fn `UserConstructionScript`)