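; AI controller for NPCs that runs BT_NPC and uses AI perception to detect the player's fox character.
; Perception updates from the Player-tagged fox go to sight and hearing handlers, which filter by sense class and write Blackboard keys.
; Sight sets the target and toggles player detection, playing an alert when seen and storing last location when lost.
; Hearing stores the sound location; HandleSense is not called here.
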(event `self.ReceiveBeginPlay`
  ; Inicializa behavior tree
  (`self.RunBehaviorTree` "/Game/FoxGame/EnemyAI/Behaiviour/BT_NPC.BT_NPC"))

(event `self.AIPerception.OnTargetPerceptionUpdated`
  (params (Actor :type "Actor Object Reference") (Stimulus :type "AIStimulus Structure"))
  ; TargetPerception, deteccion de jugador e inicializador de ui
  (bind _asbp_fox_character (cast `/Game/Characters/Fox/BP_FoxCharacter` Actor))
  (if (`self.ActorHasTag` _asbp_fox_character "Player")
    (`|ExecutionSequence`
      (:`then_0`
        (`self.HandleSight` Actor Stimulus))
      (:`then_1`
        (`self.HandleHearing` Stimulus)))))

(fn `HandleHearing`
  (params (Stimulus :type "AIStimulus Structure (by ref)"))
  (`KismetSystemLibrary.PrintString` "no esta sordo")
  (bind _returnvalue (`AIPerceptionSystem.GetSenseClassForStimulus` Stimulus))
  (if (== _returnvalue "/Script/AIModule.AISense_Hearing")
    (`KismetSystemLibrary.PrintString` "STOP YOU'VE VIOLATED THE LAW")
    (`BlackboardComponent.SetValueAsVector` (`self.Blackboard`) "SoundLocation" (`.StimulusLocation` (break `AIStimulus` (`local.Stimulus`))))
    (else
      (`KismetSystemLibrary.PrintString` "MUST HAVE BEEN THE WIN"))))

(fn `HandleSense`
  (params (InString :type String) (Stimul :type "AIStimulus Structure") (`Sensed Actor` :type "Actor Object Reference"))
  (bind (_stimul_age _stimul_expirationage _stimul_strength _stimul_stimuluslocation _stimul_receiverlocation _stimul_tag _stimul_bsuccessfullysensed) (break `AIStimulus` (`local.Stimul`)))
  ; BlackBoardBoolCall
  (`KismetSystemLibrary.PrintString` InString)
  (`BlackboardComponent.SetValueAsBool` (`self.Blackboard`) "Investigating" _stimul_bsuccessfullysensed)
  (if _stimul_bsuccessfullysensed
    ; PlayerDetection and RunSpeed
    (if (== (`local.Sensed Actor`) (`GameplayStatics.GetPlayerCharacter` 0))
      (bind _asbp_fox_character (cast `/Game/Characters/Fox/BP_FoxCharacter` (`local.Sensed Actor`)))
      (`/Game/Characters/Fox/BP_FoxCharacter.StartDetection` _asbp_fox_character true)
      (`KismetSystemLibrary.PrintString` "sensed player")
      (`BlackboardComponent.SetValueAsObject` (`self.Blackboard`) "TargetLocationActor" (`KismetMathLibrary.SelectObject` (`GameplayStatics.GetPlayerCharacter` 0) null _stimul_bsuccessfullysensed))
      (if (not _stimul_bsuccessfullysensed)
        (`BlackboardComponent.SetValueAsVector` (`self.Blackboard`) "LocationV" _stimul_stimuluslocation))
      (else
        (return)))))

(fn `HandleSight`
  (params (Actor :type "Actor Object Reference") (stimulus :type "AIStimulus Structure"))
  (bind (_stimulus_age _stimulus_expirationage _stimulus_strength _stimulus_stimuluslocation _stimulus_receiverlocation _stimulus_tag _stimulus_bsuccessfullysensed) (break `AIStimulus` (`local.stimulus`)))
  (bind _returnvalue (`AIPerceptionSystem.GetSenseClassForStimulus` stimulus))
  (`KismetSystemLibrary.PrintString` "DETECTADO")
  (if (== _returnvalue "/Script/AIModule.AISense_Sight")
    (if (== (`local.Actor`) (`GameplayStatics.GetPlayerCharacter` 0))
      (`KismetSystemLibrary.PrintString` "ES EL JUGADOR")
      (bind _asbp_fox_character (cast `/Game/Characters/Fox/BP_FoxCharacter` (`local.Actor`)))
      (`/Game/Characters/Fox/BP_FoxCharacter.StartDetection` _asbp_fox_character true)
      (`BlackboardComponent.SetValueAsObject` (`self.Blackboard`) "TargetLocationActor" (`KismetMathLibrary.SelectObject` (`GameplayStatics.GetPlayerCharacter` 0) null _stimulus_bsuccessfullysensed))
      (`KismetSystemLibrary.PrintString` "TE PERSIGO")
      (if _stimulus_bsuccessfullysensed
        (`GameplayStatics.PlaySoundAtLocation` "/Game/Audio/Guards/Detected/SQ_Detected.SQ_Detected" (`self.K2_GetActorLocation` _asbp_fox_character) (struct) 1.0 1.0 0.0 null null null null)
        (else
          (`BlackboardComponent.SetValueAsVector` (`self.Blackboard`) "LocationV" _stimulus_stimuluslocation)
          (`KismetSystemLibrary.PrintString` "ULTIMO LUGAR DONDE ESTUVE")
          (bind _asbp_fox_character_2 (cast `/Game/Characters/Fox/BP_FoxCharacter` (`local.Actor`)))
          (`/Game/Characters/Fox/BP_FoxCharacter.StartDetection` _asbp_fox_character_2 false)))
      (else
        (return)))
    (else
      (return))))

(fn `UserConstructionScript`)