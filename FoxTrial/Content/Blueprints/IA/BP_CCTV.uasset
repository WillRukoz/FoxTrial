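; Security camera that watches for Detectable actors entering its vision cone, ignoring new overlaps while the fox player is in its SafeArea.
; When idle, it sweeps in 45-degree yaw steps using nested FlipFlops, RInterpTo and timed pauses.
; During detection, Tick runs line traces that either rotate it toward the detected actor or emit noise and an alarm at the fox.
; Interact disables it once with lightning, removing cone and spotlight and tilting it via timeline.
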(event `self.ReceiveTick`
  (params (DeltaSeconds :type "Float (single-precision)"))
  (bind _as_bp_fox_character (`self.As BP Fox Character`))
  (bind _staticmesh (`self.StaticMesh`))
  (bind _returnvalue (`self.K2_GetActorLocation` _as_bp_fox_character))
  (bind (_returnvalue_roll _returnvalue_pitch _returnvalue_yaw) (`KismetMathLibrary.BreakRotator` (`SceneComponent.K2_GetComponentRotation` (`self.StaticMesh`))))
  (bind _returnvalue_x (`KismetMathLibrary.BreakVector` (`KismetMathLibrary.Conv_RotatorToVector` (`KismetMathLibrary.NormalizedDeltaRotator` (`SceneComponent.K2_GetComponentRotation` (`self.StaticMesh`)) (`self.TargetRotation`)))))
  (bind _asbp_fox_character (cast `/Game/Characters/Fox/BP_FoxCharacter` (`GameplayStatics.GetPlayerCharacter` 0)))
  (set `self.As BP Fox Character` _asbp_fox_character)
  (if (`self.IsInArea`)
    (`self.TraceCheck`
      (:`true`
        (`self.Rotate`)
        (`KismetSystemLibrary.PrintString` "no te mate"))
      (:`false`
        (`self.MakeNoise` 1.0 _as_bp_fox_character _returnvalue)
        (`GameplayStatics.PlaySoundAtLocation` "/Game/Blueprints/IA/Sound/alarm_Cue.alarm_Cue" _returnvalue (struct) 1.0 1.0 0.0 null null null null)))
    (elif (not (`self.IsDestroy?`))
      (`|ExecutionSequence`
        (:`then_0`
          (`/Engine/EditorBlueprintResources/StandardMacros.DoOnce` false :!label _label
            (:`Completed`
              (`/Engine/EditorBlueprintResources/StandardMacros.FlipFlop`
                (:`A`
                  (`/Engine/EditorBlueprintResources/StandardMacros.FlipFlop`
                    (:`A`
                      (set `self.TargetRotation` (`KismetMathLibrary.MakeRotator` _returnvalue_roll _returnvalue_pitch (+ _returnvalue_yaw 45.0)) :!label _label_2))
                    (:`B`
                      (set `self.TargetRotation` (`KismetMathLibrary.MakeRotator` _returnvalue_roll _returnvalue_pitch (- _returnvalue_yaw 45.0)) :!label _label_3))))
                (:`B`
                  (`/Engine/EditorBlueprintResources/StandardMacros.FlipFlop`
                    (:`A`
                      (goto _label_3))
                    (:`B`
                      (goto _label_2))))))))
        (:`then_1`
          (`SceneComponent.K2_SetWorldRotation` _staticmesh (`KismetMathLibrary.RInterpTo` (`SceneComponent.K2_GetComponentRotation` _staticmesh) (`self.TargetRotation`) (`GameplayStatics.GetWorldDeltaSeconds`) (`self.RotationSpeed`)) false false)
          (if (> _returnvalue_x 0.9)
            (`KismetSystemLibrary.Delay` (`self.CameraRate`))
            (goto _label :!via `Reset`)))))))

(event `self.Cone.OnComponentBeginOverlap`
  (params (OverlappedComponent :type "PrimitiveComponent Object Reference") (OtherActor :type "Actor Object Reference") (OtherComp :type "PrimitiveComponent Object Reference") (OtherBodyIndex :type Integer) (bFromSweep :type Boolean) (SweepResult :type "HitResult Structure (by ref)"))
  (if (and (not (`self.SafeArea`)) (`self.ActorHasTag` OtherActor "Detectable"))
    (set `self.DetectedActor` OtherActor)
    (set `self.IsInArea` true)))

(event `self.Cone.OnComponentEndOverlap`
  (params (OverlappedComponent :type "PrimitiveComponent Object Reference") (OtherActor :type "Actor Object Reference") (OtherComp :type "PrimitiveComponent Object Reference") (OtherBodyIndex :type Integer))
  (if (`self.ActorHasTag` OtherActor "Detectable")
    (set `self.DetectedActor` OtherActor)
    (set `self.IsInArea` false)))

(event `self.Safe Area.OnComponentBeginOverlap`
  (params (OverlappedComponent :type "PrimitiveComponent Object Reference") (OtherActor :type "Actor Object Reference") (OtherComp :type "PrimitiveComponent Object Reference") (OtherBodyIndex :type Integer) (bFromSweep :type Boolean) (SweepResult :type "HitResult Structure (by ref)"))
  (cast `/Game/Characters/Fox/BP_FoxCharacter` OtherActor)
  (set `self.SafeArea` true))

(event `self.Safe Area.OnComponentEndOverlap`
  (params (OverlappedComponent :type "PrimitiveComponent Object Reference") (OtherActor :type "Actor Object Reference") (OtherComp :type "PrimitiveComponent Object Reference") (OtherBodyIndex :type Integer))
  (cast `/Game/Characters/Fox/BP_FoxCharacter` OtherActor)
  (set `self.SafeArea` false))

(event `self.ReceiveBeginPlay`
  ; Player Ref
  (bind _asbp_fox_character (cast `/Game/Characters/Fox/BP_FoxCharacter` (`GameplayStatics.GetPlayerCharacter` 0)))
  (set `self.As BP Fox Character` _asbp_fox_character))

(event `/Game/FoxGame/LevelDesing/BPI_InterectInterface.Interact`
  (bind _staticmesh (`self.StaticMesh`))
  (bind (_returnvalue_roll _returnvalue_pitch _returnvalue_yaw) (`KismetMathLibrary.BreakRotator` (`SceneComponent.K2_GetComponentRotation` _staticmesh)))
  (`/Engine/EditorBlueprintResources/StandardMacros.DoOnce` false
    (:`Completed`
      (`GameplayStatics.PlaySoundAtLocation` "/Game/StylizedVFX-Electric/Sound/magic_spell_electro_04.magic_spell_electro_04" (`self.K2_GetActorLocation` (`self.As BP Fox Character`)) (struct) 1.0 1.0 0.0 null null null null)
      (`NiagaraFunctionLibrary.SpawnSystemAtLocation` "/Game/StylizedVFX-Electric/VFX/System/5x5/N_LightningBurst5x5_6.N_LightningBurst5x5_6" (`SceneComponent.K2_GetComponentLocation` (`self.StaticMesh`)))
      (`ActorComponent.K2_DestroyComponent` (`self.Cone`))
      (`ActorComponent.K2_DestroyComponent` (`self.SpotLight`))
      (set `self.IsDestroy?` true)
      (bind (_direction _newtrack_0) (`Timeline|camera down`)
        (:`Update`
          (`SceneComponent.K2_SetWorldRotation` _staticmesh (`KismetMathLibrary.MakeRotator` _returnvalue_roll _newtrack_0 _returnvalue_yaw) false false))))))

(fn `UserConstructionScript`)