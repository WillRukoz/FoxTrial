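; BP_StaticCamera is a one-shot trigger that briefly shows a static camera view, then returns to the fox player.
; Overlap caches the BP_FoxCharacter, while Tick polls the JugadorCerca (player nearby) flag on BPCameraDestroy.
; Once the flag is set and Camera is valid, a DoOnce switches the view target to Camera.
; After a short delay, the view returns to the cached fox and the actor destroys itself.
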(event `self.ReceiveTick`
  (params (DeltaSeconds :type "Float (single-precision)"))
  (bind _returnvalue (`GameplayStatics.GetPlayerController` 0))
  (if (`/Game/FoxGame/LevelDesing/BP_CameraDestroy.bJugadorCerca` (`self.BP_CameraDestroy`))
    (`self.Camera`
      (:`then`
        (`/Engine/EditorBlueprintResources/StandardMacros.DoOnce` false
          (:`Completed`
            (`PlayerController.SetViewTargetWithBlend` _returnvalue (`self.Camera`) 0.0 "VTBlend_Linear" 0.0 false)
            (`KismetSystemLibrary.Delay` 1.0)
            (`PlayerController.SetViewTargetWithBlend` _returnvalue (`self.As BP Fox Character`) 0.0 "VTBlend_Linear" 0.0 false)
            (`self.K2_DestroyActor`))))
      (:`else`))))

(event `self.ReceiveActorBeginOverlap`
  (params (OtherActor :type "Actor Object Reference"))
  (bind _asbp_fox_character (cast `/Game/Characters/Fox/BP_FoxCharacter` OtherActor))
  (set `self.As BP Fox Character` _asbp_fox_character))

(fn `UserConstructionScript`)