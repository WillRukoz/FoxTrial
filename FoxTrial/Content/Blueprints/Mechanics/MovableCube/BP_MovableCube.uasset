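; Movable cube that the fox character pushes or pulls while interacting within its trigger volume.
; Overlaps on the Fwr component toggle the character's CanInteractBox flag, with no filter on the overlapping actor.
; Tick fetches the character and feeds its input signs to SpeedDirection.
; That function interpolates the Cube's relative location without sweep, using its right vector for forward/back and forward vector for left/right.
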(event `self.ReceiveTick`
  (params (DeltaSeconds :type "Float (single-precision)"))
  (bind _char_ref (`self.Char Ref`))
  (bind _char_ref_2 (`self.Char Ref`))
  (bind _forward__backwards (`/Game/Characters/Fox/BP_FoxCharacter.Forward/ Backwards` _char_ref_2))
  (bind _right_left (`/Game/Characters/Fox/BP_FoxCharacter.Right/Left` _char_ref_2))
  (bind _returnvalue (`GameplayStatics.GetActorOfClass` "/Game/Characters/Fox/BP_FoxCharacter.BP_FoxCharacter_C"))
  (set `self.Char Ref` _returnvalue)
  (if (`/Game/Characters/Fox/BP_FoxCharacter.IsInteractingBox?` _char_ref)
    (if (`/Game/Characters/Fox/BP_FoxCharacter.CanInteractBox?` _char_ref)
      (`|ExecutionSequence`
        (:`then_0`
          (if (== _forward__backwards 0.0)
            (`KismetSystemLibrary.PrintString` "Players not moving Fordward or Backwards")
            (elif (>= _forward__backwards 0.1)
              (`KismetSystemLibrary.PrintString` "Players moving Fordward")
              (`self.Speed/Direction` true 50.0)
              (else
                (`KismetSystemLibrary.PrintString` "Players moving  Backwards")
                (`self.Speed/Direction` true -50.0)))))
        (:`then_1`
          (if (== _right_left 0.0)
            (`KismetSystemLibrary.PrintString` "Players not moving Fordward or Backwards")
            (elif (>= _right_left 0.1)
              (`KismetSystemLibrary.PrintString` "Players moving Right")
              (`self.Speed/Direction` false -50.0)
              (else
                (`KismetSystemLibrary.PrintString` "Players moving  Left")
                (`self.Speed/Direction` false 50.0)))))))))

(event `self.Fwr.OnComponentBeginOverlap`
  (params (OverlappedComponent :type "PrimitiveComponent Object Reference") (OtherActor :type "Actor Object Reference") (OtherComp :type "PrimitiveComponent Object Reference") (OtherBodyIndex :type Integer) (bFromSweep :type Boolean) (SweepResult :type "HitResult Structure (by ref)"))
  (`KismetSystemLibrary.PrintString` "Can Interact" true true (struct :`R` 1.0 :`G` 0.214236 :`A` 1.0) 2.0 "432342")
  (set `/Game/Characters/Fox/BP_FoxCharacter.CanInteractBox?` true (`self.Char Ref`)))

(event `self.Fwr.OnComponentEndOverlap`
  (params (OverlappedComponent :type "PrimitiveComponent Object Reference") (OtherActor :type "Actor Object Reference") (OtherComp :type "PrimitiveComponent Object Reference") (OtherBodyIndex :type Integer))
  (`KismetSystemLibrary.PrintString` "Cant Interact" true true (struct :`R` 1.0 :`G` 0.214236 :`A` 1.0) 2.0 "432342")
  (set `/Game/Characters/Fox/BP_FoxCharacter.CanInteractBox?` false (`self.Char Ref`)))

(fn `UserConstructionScript`)