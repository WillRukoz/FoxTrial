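; Cage prop that swings its door open when a BP_FoxCharacter enters its box trigger, with apparent logic to release a fox baby.
; Overlap toggles the Interact component's visibility, and the Abrir timeline rotates Puerta's yaw without any input check.
; Each door update casts that same overlapping actor to BP_FoxBaby; on success it plays a running animation and a second timeline nudges it along X.
; IsOpen is set only inside that second timeline.
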(event `self.Box.OnComponentBeginOverlap`
  (params (OverlappedComponent :type "PrimitiveComponent Object Reference") (OtherActor :type "Actor Object Reference") (OtherComp :type "PrimitiveComponent Object Reference") (OtherBodyIndex :type Integer) (bFromSweep :type Boolean) (SweepResult :type "HitResult Structure (by ref)"))
  (`SceneComponent.SetVisibility` (`self.Interact`) true false)
  (cast `/Game/Characters/Fox/BP_FoxCharacter` OtherActor)
  (if (not (`self.IsOpen`))
    (bind (_direction _rotacion) (`Timeline|Abrir`)
      (:`Update`
        (`SceneComponent.K2_SetRelativeRotation` (`self.Puerta`) (`KismetMathLibrary.MakeRotator` 0.0 0.0 _rotacion) false false)
        (bind _asbp_fox_baby (cast `/Game/Characters/Fox/BabyFox/BP_FoxBaby` OtherActor))
        (bind _returnvalue_x (`KismetMathLibrary.BreakVector` (`self.GetActorForwardVector` _asbp_fox_baby)))
        (bind _returnvalue (* _returnvalue_x 1.0))
        (`KismetSystemLibrary.PrintString` "Hello" true true (struct :`G` 0.66 :`B` 1.0 :`A` 1.0) _returnvalue)
        (`SkeletalMeshComponent.PlayAnimation` (`Character.Mesh` _asbp_fox_baby) "/Game/Characters/Fox/Animations/AS_Dog_Locomotion_Running.AS_Dog_Locomotion_Running" true)
        (`Timeline|Timeline`
          (:`Update`
            (`self.K2_AddActorWorldOffset` _asbp_fox_baby (`KismetMathLibrary.MakeVector` _returnvalue) false false)
            (set `self.IsOpen` true)))))))

(event `self.Box.OnComponentEndOverlap`
  (params (OverlappedComponent :type "PrimitiveComponent Object Reference") (OtherActor :type "Actor Object Reference") (OtherComp :type "PrimitiveComponent Object Reference") (OtherBodyIndex :type Integer))
  (`SceneComponent.SetVisibility` (`self.Interact`) false false))

(fn `UserConstructionScript`)